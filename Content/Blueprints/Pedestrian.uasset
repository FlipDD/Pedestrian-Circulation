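; Pedestrian Blueprint that logs its X position over time to a file named after the actor's display name.
; From BeginPlay, a self-looping one-second delay appends a comma-separated X location and game time string to the Data array.
; Each pass then hands the whole accumulated array to SaveStringToFile, so saving happens every second while it runs.
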(event `self.ReceiveBeginPlay`
  (bind _returnvalue_x (`KismetMathLibrary.BreakVector` (`self.K2_GetActorLocation`)))
  (bind _data (`self.Data`))
  ;[1 1 1] Add the string to the array
  (`KismetArrayLibrary.Array_Add` _data (`KismetStringLibrary.Concat_StrStr` (`KismetStringLibrary.Concat_StrStr` (`KismetStringLibrary.Conv_DoubleToString` _returnvalue_x) ", ") (`KismetStringLibrary.Conv_DoubleToString` (`KismetSystemLibrary.GetGameTimeInSeconds`))) :!label _label)
  ;[1 1 1] Save to file every 1 second
  (`UBPFL_FileIO.SaveStringToFile` _data (`KismetSystemLibrary.GetDisplayName` self))
  (`KismetSystemLibrary.Delay` 1.0)
  (goto _label))

(fn `UserConstructionScript`)